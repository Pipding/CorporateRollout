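; BP_OfficeTile is an office floor tile for a runner game where a boulder chases the player.
; Construction usually spawns one obstacle as a child actor, slightly favouring jumps over ducks because ducking slows the runner.
; It also rolls weighted chances for office props, placed as HISM instances at random child-component locations.
; When the runner overlaps EndTrigger, the game mode adds another tile and this one destroys itself after a delay.
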(event `self.EndTrigger.OnComponentBeginOverlap`
  (params (OverlappedComponent :type "PrimitiveComponent Object Reference") (OtherActor :type "Actor Object Reference") (OtherComp :type "PrimitiveComponent Object Reference") (OtherBodyIndex :type Integer) (bFromSweep :type Boolean) (SweepResult :type "HitResult Structure (by ref)"))
  ;[1 1 1] When the player reaches the end of a floor tile, spawn a new one and destroy the tile we just passed
  (cast `/Game/Characters/RunnerCharacter/BP_RunnerCharacter` OtherActor)
  (bind _asbp_runner_game_mode (cast `/Game/GameMode/BP_RunnerGameMode` (`GameplayStatics.GetGameMode`)))
  (`/Game/GameMode/BP_RunnerGameMode.AddFloorTile` _asbp_runner_game_mode)
  (`KismetSystemLibrary.Delay` 10.0)
  (`self.K2_DestroyActor`))

(fn `GetAttachTransform`
  (returns (ReturnValue :type "Transform Structure"))
  (return (`SceneComponent.K2_GetComponentToWorld` (`self.AttachPoint`))))

(fn `SetSpawnPoints`
  (set `self.ObstacleSpawnPoints` (`|MakeArray` (`SceneComponent.GetRelativeTransform` (`self.ObstacleSpawnPoint`)))))

(fn `SpawnObstacle`
  ;[1 1 1] Ducking slows the player down, making it more likely the boulder will catch up. Counteract this by slightly favouring spawning obstacles to jump over (which doesn't slow the character down)
  (if (`KismetMathLibrary.RandomBoolWithWeight` 0.6)
    (`AddComponent|NODE_AddChildActorComponent-0` :`RelativeTransform` (`KismetArrayLibrary.Array_Random` (`self.ObstacleSpawnPoints`)))
    (else
      (`AddComponent|NODE_AddChildActorComponent-1` :`RelativeTransform` (`KismetArrayLibrary.Array_Random` (`self.ObstacleSpawnPoints`))))))

(fn `SpawnProps`
  (`self.SpawnPropWithWeight` "/Game/Props/WaterCooler/WaterCooler.WaterCooler" (`self.WaterCoolerSpawnLocations`) 0.4)
  (`self.SpawnPropWithWeight` "/Game/Props/WallClock/SM_WallClock.SM_WallClock" (`self.ClockSpawnLocations`) 0.7)
  (`self.SpawnPropWithWeight` "/Game/Props/CardboardBox/CardboardBox.CardboardBox" (`self.CardboardBoxSpawnLocations`) 0.8)
  (`self.SpawnPropWithWeight` "/Game/Props/Desk/FullDesk.FullDesk" (`self.DeskSpawnLocations`) 0.5))

(fn `SpawnPropWithWeight`
  (params (PropMesh :type "StaticMesh Object Reference") (SpawnPoints :type "SceneComponent Object Reference") (SpawnChance :type "Float (single-precision)"))
  (if (`KismetMathLibrary.RandomBoolWithWeight` SpawnChance)
    (bind _returnvalue (`AddComponent|NODE_AddHierarchicalInstancedStaticMeshComponent-3`))
    (`StaticMeshComponent.SetStaticMesh` _returnvalue PropMesh)
    (`InstancedStaticMeshComponent.AddInstance` _returnvalue (`self.GetTransformOfRandomChildComponent` SpawnPoints) false)))

(fn `UserConstructionScript`
  (`self.SetSpawnPoints`) ; TODO: This can likely be optimized away
  ;[1 1 1] 95% chance to spawn an obstacle. 100% makes the game feel too predictable
  (if (`KismetMathLibrary.RandomBoolWithWeight` 0.95)
    (`self.SpawnObstacle`))
  (`self.SpawnProps`))