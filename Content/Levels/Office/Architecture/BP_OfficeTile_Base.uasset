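; Base office floor tile for an endless runner, which requests the next tile from the game mode when the runner overlaps its end trigger.
; After a delay the passed tile destroys itself, unless the player is dead.
; If obstacle spawn points exist, construction randomly adds a jump or duck obstacle, favouring jumps, and occasionally a powerup.
; A weighted instanced-mesh prop helper exists, but its calls in SpawnProps are disconnected.
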(event `self.EndTrigger.OnComponentBeginOverlap`
  (params (OverlappedComponent :type "PrimitiveComponent Object Reference") (OtherActor :type "Actor Object Reference") (OtherComp :type "PrimitiveComponent Object Reference") (OtherBodyIndex :type Integer) (bFromSweep :type Boolean) (SweepResult :type "HitResult Structure (by ref)"))
  ;[1 1 1] When the player reaches the end of a floor tile, spawn a new one and destroy the tile we just passed
  (cast `/Game/Characters/RunnerCharacter/BP_RunnerCharacter` OtherActor)
  (bind _asbp_runner_game_mode (cast `/Game/GameMode/BP_RunnerGameMode` (`GameplayStatics.GetGameMode`)))
  (`/Game/GameMode/BP_RunnerGameMode.AddFloorTile` _asbp_runner_game_mode)
  (`KismetSystemLibrary.Delay` 15.0)
  ;;[1 1 1] Tile should not despawn if the player is dead. If player is dead they are viewing the game over screen and may see tiles disappearing in the background
  (bind _asbp_runner_character (cast `/Game/Characters/RunnerCharacter/BP_RunnerCharacter` (`GameplayStatics.GetPlayerPawn` 0)))
  (if (`/Game/Characters/RunnerCharacter/BP_RunnerCharacter.IsAlive` _asbp_runner_character)
    (`self.K2_DestroyActor`)))

(fn `GetAttachTransform`
  (returns (ReturnValue :type "Transform Structure"))
  (return (`SceneComponent.K2_GetComponentToWorld` (`self.AttachPoint`))))

(fn `SpawnObstacle`
  ;[1 1 1] Ducking slows the player down, making it more likely the boulder will catch up. Counteract this by slightly favouring spawning obstacles to jump over (which doesn't slow the character down)
  (if (`KismetMathLibrary.RandomBoolWithWeight` 0.6)
    (`AddComponent|NODE_AddChildActorComponent-0` :`RelativeTransform` (`self.GetTransformOfRandomChildComponent` (`self.ObstacleSpawnPoints`)))
    (else
      (`AddComponent|NODE_AddChildActorComponent-1` :`RelativeTransform` (`self.GetTransformOfRandomChildComponent` (`self.ObstacleSpawnPoints`))))))

(fn `SpawnPowerup`
  (`AddComponent|NODE_AddChildActorComponent-4` :`RelativeTransform` (`KismetMathLibrary.MakeTransform` (`KismetMathLibrary.MakeVector` (+ (* (`KismetMathLibrary.RandomFloat`) 800.0) 100.0) 0.0 (`self.PowerupSpawnHeight`)))))

(fn `SpawnProps`)

(fn `SpawnPropWithWeight`
  (params (PropMesh :type "StaticMesh Object Reference") (SpawnPoints :type "SceneComponent Object Reference") (SpawnChance :type "Float (single-precision)"))
  (if (`KismetMathLibrary.RandomBoolWithWeight` SpawnChance)
    (bind _returnvalue (`AddComponent|NODE_AddHierarchicalInstancedStaticMeshComponent-3`))
    (`StaticMeshComponent.SetStaticMesh` _returnvalue PropMesh)
    (`InstancedStaticMeshComponent.AddInstance` _returnvalue (`self.GetTransformOfRandomChildComponent` SpawnPoints) false)))

(fn `UserConstructionScript`
  (`self.AreObstacleSpawnPointsDefined`
    (:`yes`
      ;[1 1 1] 95% chance to spawn an obstacle. 100% makes the game feel too predictable
      (if (`KismetMathLibrary.RandomBoolWithWeight` 0.95)
        (`self.SpawnObstacle`))
      (`self.SpawnProps`)
      ;[1 1 1] 10% chance to spawn a powerup
      (if (`KismetMathLibrary.RandomBoolWithWeight` 0.1)
        (`self.SpawnPowerup`)))))