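; BP_OfficeTile_Start is the starting office level tile for a runner game, with a destructible wall.
; Fifteen seconds after BeginPlay it destroys itself, but only if the player's BP_RunnerCharacter is still alive at that moment.
; Any overlap on the wall's collider plays a quieter, lower-pitched smash sound at the wall's location.
; GetAttachTransform exposes the AttachPoint world transform, presumably for chaining the next tile.
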(event `self.ReceiveBeginPlay`
  ;[1 1 1] This tile self-destructs after 15 seconds if the player is alive
  (`KismetSystemLibrary.Delay` 15.0)
  (bind _asbp_runner_character (cast `/Game/Characters/Salaryman/BP_RunnerCharacter` (`GameplayStatics.GetPlayerPawn` 0)))
  (if (`/Game/Characters/Salaryman/BP_RunnerCharacter.IsAlive` _asbp_runner_character)
    (`self.K2_DestroyActor`)))

(event `self.DestructibleWallCollider.OnComponentBeginOverlap`
  (params (OverlappedComponent :type "PrimitiveComponent Object Reference") (OtherActor :type "Actor Object Reference") (OtherComp :type "PrimitiveComponent Object Reference") (OtherBodyIndex :type Integer) (bFromSweep :type Boolean) (SweepResult :type "HitResult Structure (by ref)"))
  (`GameplayStatics.PlaySoundAtLocation` "/Game/Audio/SFX/Boulder/WallSmashSFX.WallSmashSFX" (`SceneComponent.K2_GetComponentLocation` (`self.DestructibleWall`)) (struct) 0.4 0.7 0.0 null null null null))

(fn `GetAttachTransform`
  (returns (ReturnValue :type "Transform Structure"))
  (return (`SceneComponent.K2_GetComponentToWorld` (`self.AttachPoint`))))

(fn `UserConstructionScript`)