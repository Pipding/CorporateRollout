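; BP_Obstacle is a runner-game obstacle that awards points through a score collider and punishes the runner on collision.
; Overlapping ScoreCollider adds PointValue to the score via BP_RunnerGameMode.
; Two collision handler events make BP_RunnerCharacter trip or hit its head, then explode and destroy the obstacle after a short delay; this graph does not call them.
; Explode removes both colliders to prevent repeat triggers, hides the mesh and plays smoke effects.
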(event `self.ScoreCollider.OnComponentBeginOverlap`
  (params (OverlappedComponent :type "PrimitiveComponent Object Reference") (OtherActor :type "Actor Object Reference") (OtherComp :type "PrimitiveComponent Object Reference") (OtherBodyIndex :type Integer) (bFromSweep :type Boolean) (SweepResult :type "HitResult Structure (by ref)"))
  ;[1 0.1615 0.1615] Collision events
  ;;[0.05098 0.05098 0.05098] On ScoreCollider Overlap
  (`self.GainScore`))

(event `HandleCollisionTrip`
  (params (OtherActor :type "Actor Object Reference"))
  ;[1 0.1615 0.1615] Collision events
  ;;[0.05098 0.05098 0.05098] Trip
  (bind _asbp_runner_character (cast `/Game/Characters/Salaryman/BP_RunnerCharacter` OtherActor)
    (:`then`
      (`/Game/Characters/Salaryman/BP_RunnerCharacter.Trip` _asbp_runner_character))
    (:`CastFailed`
      _))
  (`self.Explode`)
  (`KismetSystemLibrary.Delay` 0.2)
  (`self.K2_DestroyActor`))

(event `HandleCollisionHitHead`
  (params (OtherActor :type "Actor Object Reference"))
  ;[1 0.1615 0.1615] Collision events
  ;;[0.05098 0.05098 0.05098] Hit head
  (bind _asbp_runner_character (cast `/Game/Characters/Salaryman/BP_RunnerCharacter` OtherActor)
    (:`then`
      (`/Game/Characters/Salaryman/BP_RunnerCharacter.HitHead` _asbp_runner_character))
    (:`CastFailed`
      _))
  (`self.Explode`)
  (`KismetSystemLibrary.Delay` 0.2)
  (`self.K2_DestroyActor`))

(fn `Explode`
  ;[1 1 1] Destroy colliders so no further events can be triggered
  (`ActorComponent.K2_DestroyComponent` (`self.ScoreCollider`))
  (`ActorComponent.K2_DestroyComponent` (`self.HitCollider`))
  (`SceneComponent.SetVisibility` (`self.StaticMesh`) false false)
  ;[1 1 1] Play SFX and particles
  (`GameplayStatics.PlaySoundAtLocation` "/Game/Audio/SFX/Obstacles/SFX_SmokePuff_Cue.SFX_SmokePuff_Cue" (`SceneComponent.K2_GetComponentLocation` (`self.Scene`)) (struct) 1.0 1.0 0.0 (`self.ExplosionSFXAttenuationSettings`) null null null)
  (`ActorComponent.Activate` (`self.DestructionVFX`) false))

(fn `GainScore`
  (bind _asbp_runner_game_mode (cast `/Game/GameMode/BP_RunnerGameMode` (`GameplayStatics.GetGameMode`)))
  (`/Game/GameMode/BP_RunnerGameMode.AddScore` _asbp_runner_game_mode (`self.PointValue`)))

(fn `UserConstructionScript`)