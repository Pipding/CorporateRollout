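; BP_Obstacle_ExitSign is an exit sign obstacle for the runner character.
; When anything begins overlapping its HitCollider, it calls HitHead on the actor if that is a BP_RunnerCharacter.
; It then calls Explode and destroys itself after a short delay.
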(event `self.HitCollider.OnComponentBeginOverlap`
  (params (OverlappedComponent :type "PrimitiveComponent Object Reference") (OtherActor :type "Actor Object Reference") (OtherComp :type "PrimitiveComponent Object Reference") (OtherBodyIndex :type Integer) (bFromSweep :type Boolean) (SweepResult :type "HitResult Structure (by ref)"))
  ;[1 0.1615 0.1615] Collision events
  ;;[1 1 1] On HitCollider begin overlap
  (bind _asbp_runner_character (cast `/Game/Characters/Salaryman/BP_RunnerCharacter` OtherActor)
    (:`then`
      (`/Game/Characters/Salaryman/BP_RunnerCharacter.HitHead` _asbp_runner_character))
    (:`CastFailed`
      _))
  (`self.Explode`)
  (`KismetSystemLibrary.Delay` 0.2)
  (`self.K2_DestroyActor`))

(fn `UserConstructionScript`
  (`parent.UserConstructionScript`))