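; BP_Powerup is a spinning pickup that the runner character collects on touch.
; Tick calls RotateMesh, which yaws the root component at DegreesPerSecond, scaled by delta time.
; When the Collider overlaps a BP_RunnerCharacter, it calls PlayerCollectedPowerup on BP_RunnerGameMode and destroys itself, so any powerup effect is left to the GameMode.
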(event `self.ReceiveTick`
  (params (DeltaSeconds :type "Float (single-precision)"))
  (`self.RotateMesh` DeltaSeconds))

(event `self.Collider.OnComponentBeginOverlap`
  (params (OverlappedComponent :type "PrimitiveComponent Object Reference") (OtherActor :type "Actor Object Reference") (OtherComp :type "PrimitiveComponent Object Reference") (OtherBodyIndex :type Integer) (bFromSweep :type Boolean) (SweepResult :type "HitResult Structure (by ref)"))
  (cast `/Game/Characters/Salaryman/BP_RunnerCharacter` OtherActor) ; Continue only if the entity which collided is the player character
  ;[1 1 1] Tell the GameMode the player has collected a powerup & delete this actor
  (bind _asbp_runner_game_mode (cast `/Game/GameMode/BP_RunnerGameMode` (`GameplayStatics.GetGameMode`)))
  (`/Game/GameMode/BP_RunnerGameMode.PlayerCollectedPowerup` _asbp_runner_game_mode)
  (`self.K2_DestroyActor`))

(fn `RotateMesh`
  (params (DeltaTime :type "Float (double-precision)"))
  (bind (_returnvalue_roll _returnvalue_pitch _returnvalue_yaw) (`KismetMathLibrary.BreakRotator` (`SceneComponent.K2_GetComponentRotation` (`self.DefaultSceneRoot`))))
  (`SceneComponent.K2_SetWorldRotation` (`self.DefaultSceneRoot`) (`KismetMathLibrary.MakeRotator` _returnvalue_roll _returnvalue_pitch (+ _returnvalue_yaw (* DeltaTime (`self.DegreesPerSecond`)))) false false))

(fn `UserConstructionScript`)