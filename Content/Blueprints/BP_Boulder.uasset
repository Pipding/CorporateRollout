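; BP_Boulder is a rolling boulder hazard that chases the runner and calls Die on any BP_RunnerCharacter overlapping its collision box.
; Each Tick it moves along world +X at Speed, spinning the mesh at a fixed rate to fake rolling.
; While PursuitMode, toggled through SetPursuitMode, is on, it snaps up to MaxDistanceFromPlayer behind the player whenever it lags farther, assuming the player runs toward +X.
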(event `self.ReceiveTick`
  (params (DeltaSeconds :type "Float (single-precision)"))
  (`self.PursuePlayer` DeltaSeconds))

(event `self.Collisionbox.OnComponentBeginOverlap`
  (params (OverlappedComponent :type "PrimitiveComponent Object Reference") (OtherActor :type "Actor Object Reference") (OtherComp :type "PrimitiveComponent Object Reference") (OtherBodyIndex :type Integer) (bFromSweep :type Boolean) (SweepResult :type "HitResult Structure (by ref)"))
  (bind _asbp_runner_character (cast `/Game/Characters/RunnerCharacter/BP_RunnerCharacter` OtherActor))
  (`/Game/Characters/RunnerCharacter/BP_RunnerCharacter.Die` _asbp_runner_character))

(fn `CatchUpToPlayer`
  (bind (_returnvalue_x _returnvalue_y) (`KismetMathLibrary.BreakVector` (`self.GetPlayerLocation`)))
  (`SceneComponent.K2_SetWorldLocation` (`self.DefaultSceneRoot`) (`KismetMathLibrary.MakeVector` (- _returnvalue_x (`self.MaxDistanceFromPlayer`)) _returnvalue_y) false false))

(fn `MoveForward`
  (params (DeltaTime :type "Float (double-precision)"))
  (bind (_returnvalue_x _returnvalue_y _returnvalue_z) (`KismetMathLibrary.BreakVector` (`SceneComponent.K2_GetComponentLocation` (`self.DefaultSceneRoot`))))
  (`SceneComponent.K2_SetWorldLocation` (`self.DefaultSceneRoot`) (`KismetMathLibrary.MakeVector` (+ (* DeltaTime (`self.Speed`)) _returnvalue_x) _returnvalue_y _returnvalue_z) false false)
  (`SceneComponent.K2_AddWorldRotation` (`self.BoulderMesh`) (`KismetMathLibrary.MakeRotator` 0.0 (* (`GameplayStatics.GetWorldDeltaSeconds`) -180.0)) false false))

(fn `PursuePlayer`
  (params (DeltaTime :type "Float (double-precision)"))
  (if (and (> (`self.DistanceToPlayer`) (`self.MaxDistanceFromPlayer`)) (`self.PursuitMode`))
    (`self.CatchUpToPlayer`))
  (`self.MoveForward` DeltaTime))

(fn `SetPursuitMode`
  (params (PursuitMode :type Boolean))
  (set `self.PursuitMode` PursuitMode))

(fn `UserConstructionScript`)