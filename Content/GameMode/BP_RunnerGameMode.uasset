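; Game mode for a runner game that manages score, the start countdown, powerup UI and game over.
; On BeginPlay it spawns floor tiles chained by each tile's attach transform.
; Tick adds score while the player is enabled and alive, AddScore shows timed bonus popups, and death registers the score with RunnerGameInstance.
; Level blueprints trigger widget creation and the countdown, which enables the player character on "GO!".
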(event `SpawnPowerupGetWidget`
  ;[1 1 1] Events for spawning UI widgets. These are triggered from the level blueprint, allowing different levels to enable/disable UI elements
  (`self.CreatePowerupGainedWidget`))

(event `SpawnPowerupCounterWidget`
  ;[1 1 1] Events for spawning UI widgets. These are triggered from the level blueprint, allowing different levels to enable/disable UI elements
  (`self.CreatePowerupCounterWidget`))

(event `SpawnScoreGainedWidget`
  ;[1 1 1] Events for spawning UI widgets. These are triggered from the level blueprint, allowing different levels to enable/disable UI elements
  (`self.CreateScoreGainedWidget`))

(event `SpawnScoreWidget`
  ;[1 1 1] Events for spawning UI widgets. These are triggered from the level blueprint, allowing different levels to enable/disable UI elements
  (`self.CreateScoreWidget`))

(event `self.ReceiveBeginPlay`
  ;[1 1 1] Begin play
  (`self.SpawnInitialFloorTiles`))

(event `self.ReceiveTick`
  (params (DeltaSeconds :type "Float (single-precision)"))
  ;[1 1 1] Tick
  (bind _bp_runnercharacter (`self.GetPlayerCharacter`))
  (if (and (`/Game/Characters/RunnerCharacter/BP_RunnerCharacter.IsEnabled` _bp_runnercharacter) (`/Game/Characters/RunnerCharacter/BP_RunnerCharacter.IsAlive` _bp_runnercharacter))
    (bind _newscore (`self.AddScorePerSecond` DeltaSeconds))
    (set `/Game/UI/Score/ScoreWidget.Score` _newscore (`self.ScoreWidget`))))

(event `StartCountdown`
  (`self.CreateCountdownWidget`)
  (`self.RunCountdown`))

(event `EnablePlayerCharacter`
  (bind _asbp_runner_character (cast `/Game/Characters/RunnerCharacter/BP_RunnerCharacter` (`GameplayStatics.GetPlayerCharacter` 0)))
  (`/Game/Characters/RunnerCharacter/BP_RunnerCharacter.SetIsEnabled` _asbp_runner_character true))

(event `AddScore`
  (params (Score :type "Float (double-precision)"))
  (`GameplayStatics.PlaySound2D` "/Game/Audio/SFX/ObstacleDodge/ObstacleDodgedSFX.ObstacleDodgedSFX" 1.0 1.0 0.0 null null)
  (set `self.Score` (+ Score (`self.Score`)))
  ;[1 1 1] Show score gained
  (set `/Game/UI/Score/ScoreGainedWidget.ScoreGained` Score (`self.ScoreGainedWidget`))
  (`UserWidget.AddToViewport` (`self.ScoreGainedWidget`) 0)
  (`KismetSystemLibrary.Delay` 1.0)
  (`Widget.RemoveFromParent` (`self.ScoreGainedWidget`)))

(event `PlayerDied`
  (bind _asrunner_game_instance (cast `/Game/GameMode/RunnerGameInstance` (`GameplayStatics.GetGameInstance`)))
  (`/Game/GameMode/RunnerGameInstance.RegisterNewScore` _asrunner_game_instance (`self.Score`)))

(event `GameOver`
  (`self.CreateGameOverWidget`))

(event `PlayerCollectedPowerup`
  (bind _powerupgainedwidget (`self.PowerupGainedWidget`))
  (bind _asbp_runner_character (cast `/Game/Characters/RunnerCharacter/BP_RunnerCharacter` (`GameplayStatics.GetPlayerPawn` 0)))
  (`/Game/Characters/RunnerCharacter/BP_RunnerCharacter.ObtainPowerup` _asbp_runner_character)
  ;[1 1 1] Spawn UI widgets
  (`UserWidget.AddToViewport` _powerupgainedwidget 0)
  (`UserWidget.AddToViewport` (`self.PowerupCounterWidget`) 0)
  (`KismetSystemLibrary.Delay` 2.0)
  (`Widget.RemoveFromParent` _powerupgainedwidget))

(event `PlayerUsedPowerup`
  (`Widget.RemoveFromParent` (`self.PowerupCounterWidget`)))

(fn `AddFloorTile`
  (bind _returnvalue (`|SpawnActorFromClass` "/Game/Levels/Office/Blueprints/BP_OfficeTile.BP_OfficeTile_C" (`self.NextTilePosition`) "Undefined" "MultiplyWithRoot" null null))
  (bind _returnvalue_2 (`/Game/Levels/Office/Blueprints/BP_OfficeTile.GetAttachTransform` _returnvalue))
  (set `self.NextTilePosition` _returnvalue_2))

(fn `AddScorePerSecond`
  (params (DeltaTime :type "Float (double-precision)"))
  (returns (NewScore :type "Float (double-precision)"))
  (bind _output_get (set `self.Score` (+ (* DeltaTime (`self.ScorePerSecond`)) (`self.Score`))))
  (return _output_get))

(fn `CreateCountdownWidget`
  (bind _returnvalue (`|CreateWidget` "/Game/UI/Countdown/CountdownWidget.CountdownWidget_C"))
  (bind _output_get (set `self.CountdownWidget` _returnvalue))
  (`UserWidget.AddToViewport` _output_get 0))

(fn `CreateGameOverWidget`
  (bind _returnvalue (`|CreateWidget` "/Game/UI/GameOver/GameOVerWidget.GameOverWidget_C"))
  (bind _output_get (set `self.GameOverWidget` _returnvalue))
  (`UserWidget.AddToViewport` _output_get 0))

(fn `CreatePowerupCounterWidget`
  (bind _returnvalue (`|CreateWidget` "/Game/UI/Powerups/PowerupCounterWidget.PowerupCounterWidget_C"))
  (set `self.PowerupCounterWidget` _returnvalue))

(fn `CreatePowerupGainedWidget`
  (bind _returnvalue (`|CreateWidget` "/Game/UI/Powerups/PowerupGainedWidget.PowerupGainedWidget_C"))
  (set `self.PowerupGainedWidget` _returnvalue))

(fn `CreateScoreGainedWidget`
  (bind _returnvalue (`|CreateWidget` "/Game/UI/Score/ScoreGainedWidget.ScoreGainedWidget_C"))
  (set `self.ScoreGainedWidget` _returnvalue))

(fn `CreateScoreWidget`
  (bind _returnvalue (`|CreateWidget` "/Game/UI/Score/ScoreWidget.ScoreWidget_C"))
  (set `self.ScoreWidget` _returnvalue)
  (`UserWidget.AddToViewport` (`self.ScoreWidget`) 0))

(fn `Spawn Boulder`
  (params (Transform :type "Transform Structure"))
  (bind _returnvalue (`|SpawnActorFromClass` "/Game/Levels/Office/Blueprints/BP_Boulder.BP_Boulder_C" Transform "Undefined" "MultiplyWithRoot" null null))
  (set `self.Boulder` _returnvalue))

(fn `UserConstructionScript`)